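; BP_Item is a world pickup actor that a player can interact with to add its item to their inventory.
; The construction script looks up the item's ID in DT_Item and applies that row's mesh, so each placed instance shows its configured item.
; On Interact, it passes its Item data to the player's BPCInventory component and destroys itself only if the add succeeds.
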(event EventInteract
  (params (Player :type BP%20Player%20Object%20Reference))
  (bind _succes (Default|AddtoInventory (Variables|/Game/Player/BP_Player.BP_Player_C|GetBPC_Inventory Player) (Variables|Default|GetItem)))
  (if _succes
    (Actor|DestroyActor)))

(fn ConstructionScript
  (bind _returnvalue (Utilities|GetDataTableRow "/Game/DataTables/DT_Item.DT_Item" (.RowName (Utilities|Struct|BreakDataTableRowHandle (.Item_ID (Utilities|Struct|BreakBPS_Slot (Variables|Default|GetItem))))))
    (:then
      (Components|StaticMesh|SetStaticMesh (Variables|Default|GetStaticMesh) (.mesh _returnvalue)))))