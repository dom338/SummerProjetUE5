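; BP_Money is an interactable money pickup actor whose type comes from a row in the DT_Money data table.
; The construction script looks up the selected MoneyType row and applies its mesh to the SMMoney component.
; On Interact, it adds the row's Amount to the player's MoneyAmount, prints the new total and destroys itself.
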(event EventInteract
  (params (Player :type BP%20Player%20Object%20Reference))
  (bind _returnvalue (Utilities|GetDataTableRow "/Game/DataTables/DT_Money.DT_Money" (.rowname (Variables|Default|GetMoneyType)))
    (:then
      (bind _output_get (Variables|/Game/Player/BP_Player.BP_Player_C|SetMoneyAmount Player (+ (.amount _returnvalue) (Variables|/Game/Player/BP_Player.BP_Player_C|GetMoneyAmount Player))))
      (Development|PrintString (Utilities|String|ToString(Integer) _output_get))
      (Actor|DestroyActor))))

(fn ConstructionScript
  (bind _returnvalue (Utilities|GetDataTableRow "/Game/DataTables/DT_Money.DT_Money" (.rowname (Variables|Default|GetMoneyType)))
    (:then
      (Components|StaticMesh|SetStaticMesh (Variables|Default|GetSM_Money) (.mesh _returnvalue)))))