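; BPC_Inventory is an inventory component that opens the inventory screen during play.
; On BeginPlay it creates and stores a WBP_Inventory widget, then caches the player character as BP_Player.
; The IA_OpenInventory input adds that widget to the viewport, shows the mouse cursor, pauses the game and switches to UI-only input focused on the widget.
; It contains no logic for closing the screen or storing items.
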(event Input|EnhancedActionEvents|EnhancedInputActionIA_OpenInventory
  (params (ActionValue :type Boolean) (ElapsedSeconds :type Float%20%28double-precision%29) (TriggeredSeconds :type Float%20%28double-precision%29) (InputAction :type Input%20Action%20Object%20Reference :default "/Game/Input/Actions/IA_OpenInventory.IA_OpenInventory"))
  (bind _returnvalue (Game|GetPlayerController 0))
  ;[0.15 0.15 0.15 0.5] Open Inventory
  (:Started
    (UserInterface|Viewport|AddtoViewport (Variables|Widjets|GetInventoryWidjet) 0)
    (Variables|/Script/Engine.PlayerController|SetbShowMouseCursor _returnvalue true)
    (Game|SetGamePaused true)
    (Input|SetInputModeUIOnly _returnvalue (Variables|Widjets|GetInventoryWidjet) "DoNotLock" false)))

(event EventBeginPlay
  ;[0.15 0.15 0.15 0.5] Begin Play
  (bind _returnvalue (UserInterface|CreateWidget "/Game/UI/Widjets/WBP_Inventory.WBP_Inventory_C"))
  (Variables|Widjets|SetInventoryWidjet _returnvalue)
  (bind _asbp_player (Utilities|Casting|CastToBP_Player (Game|GetPlayerCharacter 0)))
  (Variables|Player|SetAs%20BP%20Player _asbp_player))